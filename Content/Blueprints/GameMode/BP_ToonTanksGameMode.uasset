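; Game mode for ToonTanks that manages the game's UI: player HUD, start screen and game over screen.
; On BeginPlay it creates the player HUD, then each Tick polls the player tank's Health component to update the life bar.
; StartGame shows the start widget, and GameOver shows an end widget with win or lose text based on its WonGame flag.
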(event `self.ReceiveBeginPlay`
  (bind _returnvalue (`|CreateWidget` "/Game/Blueprints/Widgets/WBP_PlayerHUD.WBP_PlayerHUD_C"))
  (bind _output_get (set `self.PlayerHUDWidget` _returnvalue))
  (`UserWidget.AddToViewport` _output_get 0))

(event `self.ReceiveTick`
  (params (DeltaSeconds :type "Float (single-precision)"))
  (bind _asbp_pawn_tank (cast `/Game/Blueprints/Pawns/BP_PawnTank` (`GameplayStatics.GetPlayerPawn` 0)))
  (bind _returnvalue (`HealthComponent.GetHealth` (`/Game/Blueprints/Pawns/BP_PawnTank.Health` _asbp_pawn_tank)))
  (`/Game/Blueprints/Widgets/WBP_PlayerHUD.Update Life Bar` (`self.PlayerHUDWidget`) _returnvalue))

(event `self.StartGame`
  (bind _returnvalue (`|CreateWidget` "/Game/Blueprints/Widgets/WBP_StartGameWidget.WBP_StartGameWidget_C"))
  (`UserWidget.AddToViewport` _returnvalue 0))

(event `self.GameOver`
  (params (bWonGame :type Boolean))
  (bind _returnvalue (`|CreateWidget` "/Game/Blueprints/Widgets/WBP_GameOver.WBP_GameOver_C"))
  (`UserWidget.AddToViewport` _returnvalue 0)
  (`TextBlock.SetText` (`/Game/Blueprints/Widgets/WBP_GameOver.GameOverText` _returnvalue) (select `bool` bWonGame :`false` "You Lost!" :`true` "You Won!!!" :!type "Text")))

(fn `UserConstructionScript`)